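; BunnyBlueprintBP is a bouncing bunny actor for a BunnyMark test, with all motion logic in Blueprint.
; BeginPlay picks a random stepped Y depth and random starting speeds in the X/Z plane.
; Tick applies gravity per frame without delta time, bounces off the side bounds and damped floor with random kicks, and stops upward speed at the ceiling.
; It then sets the actor location directly without sweep.
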(event `self.ReceiveBeginPlay`
  (set `self.yf` (* (`KismetMathLibrary.FTrunc` (`KismetMathLibrary.RandomFloatInRange` 0.0 20.0)) 40.0))
  (set `self.speedXf` (* (`KismetMathLibrary.RandomFloat`) 10.0))
  (set `self.speedYf` (- (* (`KismetMathLibrary.RandomFloat`) 10.0) 5.0)))

(event `self.ReceiveTick`
  (params (DeltaSeconds :type "Float (single-precision)"))
  (set `self.xf` (+ (`self.xf`) (`self.speedXf`)))
  (set `self.zf` (- (`self.zf`) (`self.speedYf`)))
  (set `self.speedYf` (+ (`self.speedYf`) (`self.gravity`)))
  (`|ExecutionSequence`
    (:`then_0`
      (if (> (`self.xf`) (`self.maxX`))
        (set `self.speedXf` (* (`self.speedXf`) -1.0))
        (set `self.xf` (`self.maxX`))
        (elif (< (`self.xf`) (`self.minX`))
          (set `self.speedXf` (* (`self.speedXf`) -1.0))
          (set `self.xf` (`self.minX`)))))
    (:`then_1`
      (if (< (`self.zf`) (`self.minY`))
        (set `self.speedYf` (* (`self.speedYf`) -0.85))
        (set `self.zf` (`self.minY`))
        (if (> (`KismetMathLibrary.RandomFloat`) 0.5)
          (set `self.speedYf` (- (`self.speedYf`) (* (`KismetMathLibrary.RandomFloat`) 6.0))))
        (elif (> (`self.zf`) (`self.maxY`))
          (set `self.speedYf` 0.0)
          (set `self.zf` (`self.maxY`)))))
    (:`then_2`
      (`self.K2_SetActorLocation` (`KismetMathLibrary.MakeVector` (`self.xf`) (`self.yf`) (`self.zf`))))))

(fn `UserConstructionScript`)